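; Obstacle generator for the Western level that starts spawning actors at three spawner points shortly after BeginPlay.
; Tick rerolls a random selector that SpawnObstacle reads to pick one spawner or a pair.
; Each spawn waits on a delay mapped from game time, shrinking toward MaxTime.
; Spawner and Spawner1 branches call SpawnObstacle again to loop, while the Spawner2 branch ends after spawning.
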(event `self.ReceiveBeginPlay`
  ;[1 1 1] Call Obstacle on BeginPlay
  (set `self.FRandomBegin` (`KismetMathLibrary.RandomFloatInRange` 3.0 6.0))
  (`KismetSystemLibrary.Delay` 0.2)
  (`self.Spawn Obstacle`))

(event `Spawn Obstacle`
  (bind _ispawneractivate (`self.iSpawnerActivate`))
  (bind _returnvalue (`KismetMathLibrary.MapRangeClamped` (`KismetSystemLibrary.GetGameTimeInSeconds`) 0.0 (`self.MaxTime`) 3.0 1.0))
  ;[1 1 1] Spawn Obstacle with Delay that decreased with the time
  (if (< _ispawneractivate 4)
    (`KismetSystemLibrary.Delay` _returnvalue :!label _label)
    (`|SpawnActorFromClass` "/Game/Game/BP/bp_Obstacle.bp_Obstacle_C" (`SceneComponent.K2_GetComponentToWorld` (`self.Spawner`)) "Undefined" "MultiplyWithRoot" null null)
    (elif (< _ispawneractivate 7)
      (`KismetSystemLibrary.Delay` _returnvalue :!label _label_2)
      (`|SpawnActorFromClass` "/Game/Game/BP/bp_Obstacle.bp_Obstacle_C" (`SceneComponent.K2_GetComponentToWorld` (`self.Spawner1`)) "Undefined" "MultiplyWithRoot" null null)
      (else
        (if (< _ispawneractivate 10)
          _
          (elif (== _ispawneractivate 10)
            (`|ExecutionSequence`
              (:`then_0`
                (goto _label))
              (:`then_1`
                (goto _label_2)))
            (elif (== _ispawneractivate 11)
              (`|ExecutionSequence`
                (:`then_0`
                  (goto _label_2))
                (:`then_1`
                  _))
              (else
                (`|ExecutionSequence`
                  (:`then_0`
                    (goto _label))
                  (:`then_1`
                    _))))))
        (`KismetSystemLibrary.Delay` _returnvalue)
        (`|SpawnActorFromClass` "/Game/Game/BP/bp_Obstacle.bp_Obstacle_C" (`SceneComponent.K2_GetComponentToWorld` (`self.Spawner2`)) "Undefined" "MultiplyWithRoot" null null))))
  (`self.Spawn Obstacle`))

(event `self.ReceiveTick`
  (params (DeltaSeconds :type "Float (single-precision)"))
  ;[1 1 1] Set wich spawner activate
  (set `self.iSpawnerActivate` (`KismetMathLibrary.RandomIntegerInRange` 1 12)))

(fn `UserConstructionScript`)