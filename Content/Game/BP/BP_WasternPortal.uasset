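; Portal actor that switches the game from the spaceship section to the Western wagon section, expiring after a 10-second lifespan.
; When BP_Spaceship overlaps it, it destroys the obstacle manager, scrolling slide and ship, and calls DestroyObstacle on the game instance.
; After a short delay it spawns the lane wagon and a player wagon at the ship's old location, possesses the latter, destroys itself and spawns BP_WesternManager.
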(event `self.ReceiveBeginPlay`
  (`KismetSystemLibrary.PrintString` "Hello")
  (`self.SetLifeSpan` 10.0))

(event `self.PortailCollider.OnComponentBeginOverlap`
  (params (OverlappedComponent :type "PrimitiveComponent Object Reference") (OtherActor :type "Actor Object Reference") (OtherComp :type "PrimitiveComponent Object Reference") (OtherBodyIndex :type Integer) (bFromSweep :type Boolean) (SweepResult :type "HitResult Structure (by ref)"))
  (bind _old_char_pos_location (`KismetMathLibrary.BreakTransform` (`self.Old Char pos`)))
  (cast `/Game/Game/BP/BP_Spaceship` OtherActor)
  (`KismetSystemLibrary.PrintString` "portal")
  (`|ExecutionSequence`
    (:`then_1`
      (bind _returnvalue (`GameplayStatics.GetActorOfClass` "/Game/Game/BP/Bp_ObstacleManager.Bp_ObstacleManager_C"))
      (`self.K2_DestroyActor` _returnvalue))
    (:`then_2`
      (bind _asbp_game_instance (cast `/Game/Game/BP/bp_GameInstance` (`GameplayStatics.GetGameInstance`)))
      (`/Game/Game/BP/bp_GameInstance.destroyObstacle` _asbp_game_instance))
    (:`then_3`
      (bind _returnvalue_2 (`GameplayStatics.GetActorOfClass` "/Game/Game/BP/BP_Slide_scrolling.BP_Slide_scrolling_C"))
      (`self.K2_DestroyActor` _returnvalue_2))
    (:`then_4`
      (bind _returnvalue_3 (`GameplayStatics.GetActorOfClass` "/Game/Game/BP/BP_Spaceship.BP_Spaceship_C"))
      (set `self.Old Char pos` (`self.GetTransform` _returnvalue_3))
      (`self.K2_DestroyActor` _returnvalue_3)
      (`KismetSystemLibrary.Delay` 0.2)
      (`|ExecutionSequence`
        (:`then_0`
          (`|SpawnActorFromClass` "/Game/Game/BP/BP_LaneWagon.BP_LaneWagon_C" (`KismetMathLibrary.MakeTransform` (0.0 0.0 0.0) (struct :`Yaw` 90.0)) "Undefined" "MultiplyWithRoot" null null))
        (:`then_1`
          (bind _returnvalue_4 (`|SpawnActorFromClass` "/Game/Game/BP/BP_Wagon.BP_Wagon_C" (`KismetMathLibrary.MakeTransform` (+ (.location (`KismetMathLibrary.MakeTransform` _old_char_pos_location)) (0.0 0.0 0.0))) "Undefined" "MultiplyWithRoot" null null))
          (`Controller.Possess` (`GameplayStatics.GetPlayerController` 0) _returnvalue_4)
          (`KismetSystemLibrary.DelayUntilNextTick`)
          (`self.K2_DestroyActor`)
          (`|SpawnActorFromClass` "/Game/Game/BP/BP_WesternManager.BP_WesternManager_C" (`KismetMathLibrary.MakeTransform` (-500.0 -0.0 50.0) (struct :`Yaw` 90.0)) "Undefined" "MultiplyWithRoot" null null))))))

(fn `UserConstructionScript`)