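; BP_GroundGeneratorWestern is a spawner that keeps producing ground actors for the Western level.
; From BeginPlay, a self-calling SpawnGround event spawns a BP_GroundStartWesternLevel at the Generator component's transform, waits, then repeats indefinitely.
; The wait is mapped from game time up to MaxTime, but both output bounds use OutRangeA, so the interval does not vary with time.
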(event `self.ReceiveBeginPlay`
  (`self.Spawn Ground`))

(event `Spawn Ground`
  (bind _out_range_a (`self.Out Range A`))
  (`|SpawnActorFromClass` "/Game/Game/BP/Western/BP_GroundStartWesternLevel.BP_GroundStartWesternLevel_C" (`SceneComponent.K2_GetComponentToWorld` (`self.Generator`)) "Undefined" "MultiplyWithRoot" null null)
  (`KismetSystemLibrary.Delay` (`KismetMathLibrary.MapRangeClamped` (`KismetSystemLibrary.GetGameTimeInSeconds`) 0.0 (`self.Max Time`) _out_range_a _out_range_a))
  (`self.Spawn Ground`))

(fn `UserConstructionScript`)