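; Portal actor that switches the game from the spaceship phase to the snow phase when BP_Spaceship overlaps its box, and expires after a short lifespan.
; The overlap spawns and possesses a BP_SnowPlayer at the ship's transform, then destroys the ship.
; It also replaces the obstacle manager with an offset snow terrain generator, calls DestroyObstacle on the game instance and removes the slide-scrolling actor.
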(event `self.ReceiveBeginPlay`
  (`KismetSystemLibrary.PrintString` "Hello")
  (`self.SetLifeSpan` 10.0))

(event `self.Box.OnComponentBeginOverlap`
  (params (OverlappedComponent :type "PrimitiveComponent Object Reference") (OtherActor :type "Actor Object Reference") (OtherComp :type "PrimitiveComponent Object Reference") (OtherBodyIndex :type Integer) (bFromSweep :type Boolean) (SweepResult :type "HitResult Structure (by ref)"))
  (cast `/Game/Game/BP/BP_Spaceship` OtherActor)
  (`KismetSystemLibrary.PrintString` "caca")
  (`|ExecutionSequence`
    (:`then_0`
      (bind _returnvalue (`GameplayStatics.GetActorOfClass` "/Game/Game/BP/BP_Spaceship.BP_Spaceship_C"))
      (bind _returnvalue_2 (`|SpawnActorFromClass` "/Game/Game/BP/BP_SnowPlayer.BP_SnowPlayer_C" (`self.GetTransform` _returnvalue) "Undefined" "MultiplyWithRoot" null null))
      (`Controller.Possess` (`GameplayStatics.GetPlayerController` 0) _returnvalue_2)
      (`self.K2_DestroyActor` _returnvalue))
    (:`then_1`
      (bind _returnvalue_3 (`GameplayStatics.GetActorOfClass` "/Game/Game/BP/Bp_ObstacleManager.Bp_ObstacleManager_C"))
      (bind _returnvalue_4 (`self.GetTransform` _returnvalue_3))
      (`|SpawnActorFromClass` "/Game/Game/BP/BP_SnowTerrainGeneration.BP_SnowTerrainGeneration_C" (`KismetMathLibrary.MakeTransform` (`KismetMathLibrary.MakeVector` (.x (.location _returnvalue_4)) (- (.y (.location _returnvalue_4)) 1000.0) (.z (.location _returnvalue_4))) (.rotation _returnvalue_4) (.scale _returnvalue_4)) "Undefined" "MultiplyWithRoot" null null)
      (`self.K2_DestroyActor` _returnvalue_3))
    (:`then_2`
      (bind _asgi_global_variable (cast `/Game/Game/BP/GI_GlobalVariable` (`GameplayStatics.GetGameInstance`)))
      (`/Game/Game/BP/GI_GlobalVariable.destroyObstacle` _asgi_global_variable))
    (:`then_3`
      (bind _returnvalue_5 (`GameplayStatics.GetActorOfClass` "/Game/Game/BP/BP_Slide_scrolling.BP_Slide_scrolling_C"))
      (`self.K2_DestroyActor` _returnvalue_5))))

(fn `UserConstructionScript`)