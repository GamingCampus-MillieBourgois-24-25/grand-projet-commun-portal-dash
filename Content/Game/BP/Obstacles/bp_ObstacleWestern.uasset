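; Western-themed moving obstacle that ends the run when BP_Spaceship overlaps its box.
; On BeginPlay it picks one of four rock, barrel or cactus meshes with a matching transform and sets a short lifespan.
; Construction raises projectile speeds using the Speed curve sampled at game time, times a random factor.
; Overlap plays audio, sets PlayerDead, then shows UI_EndScreen after a short delay.
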(event `self.ReceiveBeginPlay`
  (bind _cube (`self.Cube`))
  (bind _cube_2 (`self.Cube`))
  (`self.SetLifeSpan` 6.0)
  (bind _output_get (set `self.iRandomObstacle` (`KismetMathLibrary.RandomIntegerInRange` 0 3)))
  (switch `int` _output_get
    (:`0`
      (`StaticMeshComponent.SetStaticMesh` _cube "/Game/Game/asset/Western/Rocks/portaldash_3d_western_rocks.portaldash_3d_western_rocks") ; Rocks
      (`SceneComponent.K2_SetRelativeLocationAndRotation` :`self` _cube_2))
    (:`1`
      (`StaticMeshComponent.SetStaticMesh` _cube "/Game/Game/asset/Western/Barrel/portaldash_3D_western_barrel.portaldash_3D_western_barrel") ; Barrel
      (`SceneComponent.K2_SetRelativeLocationAndRotation` _cube_2 (35.0 0.0 25.0) (struct :`Pitch` 90.0) false false))
    (:`2`
      (`StaticMeshComponent.SetStaticMesh` _cube "/Game/Game/asset/Western/Cactus_seul/portaldash_3d_western_cactus1.portaldash_3d_western_cactus1") ; Cactus
      (`SceneComponent.K2_SetRelativeLocationAndRotation` _cube_2 (0.0 0.0 0.0) (struct :`Yaw` 90.0) false false))
    (:`3`
      (`StaticMeshComponent.SetStaticMesh` _cube "/Game/Game/asset/Western/Cactus_+_bones_+_rocks/portaldash_3d_western_cactus+rocks+bones.portaldash_3d_western_cactus+rocks+bones") ; Cactus/Bone/Rock
      (`SceneComponent.K2_SetRelativeLocationAndRotation` :`self` _cube_2))))

(event `self.Box.OnComponentBeginOverlap`
  (params (OverlappedComponent :type "PrimitiveComponent Object Reference") (OtherActor :type "Actor Object Reference") (OtherComp :type "PrimitiveComponent Object Reference") (OtherBodyIndex :type Integer) (bFromSweep :type Boolean) (SweepResult :type "HitResult Structure (by ref)"))
  (cast `/Game/Game/BP/Space/BP_Spaceship` OtherActor)
  (`AudioComponent.Play` (`self.Audio`) 0.0)
  (set `self.PlayerDead` true)
  (`KismetSystemLibrary.Delay` 1.0)
  (bind _returnvalue (`|CreateWidget` "/Game/Game/BP/UI/UI_EndScreen.UI_EndScreen_C"))
  (`UserWidget.AddToViewport` _returnvalue 0))

(fn `UserConstructionScript`
  (bind _projectilemovement (`self.ProjectileMovement`))
  (bind _returnvalue (+ (`ProjectileMovementComponent.MaxSpeed` _projectilemovement) (* (`CurveFloat.GetFloatValue` (`self.Speed`) (`GameplayStatics.GetTimeSeconds`)) (`KismetMathLibrary.RandomFloatInRange` 150.0 200.0))))
  (set `ProjectileMovementComponent.MaxSpeed` _returnvalue _projectilemovement)
  (set `ProjectileMovementComponent.InitialSpeed` _returnvalue _projectilemovement))