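; Projectile obstacle for a spaceship game that ends the run when it hits the player.
; The construction script raises ProjectileMovement max and initial speed by a Speed curve sampled at game time and randomly scaled, with initial speed built on the raised max.
; A cube hit on BP_Spaceship plays audio, sets PlayerDead and shows UI_EndScreen after a short delay.
; Each obstacle limits its own lifetime on BeginPlay.
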(event `self.ReceiveBeginPlay`
  ;[1 1 1] Init
  (`self.SetLifeSpan` 6.0))

(event `self.Cube.OnComponentHit`
  (params (HitComponent :type "PrimitiveComponent Object Reference") (OtherActor :type "Actor Object Reference") (OtherComp :type "PrimitiveComponent Object Reference") (NormalImpulse :type "Vector Structure") (Hit :type "HitResult Structure (by ref)"))
  ;[1 1 1] Hit player
  (cast `/Game/Game/BP/Space/BP_Spaceship` OtherActor)
  (`AudioComponent.Play` (`self.Audio`) 0.0)
  (set `self.PlayerDead` true)
  (`KismetSystemLibrary.Delay` 1.0)
  (bind _returnvalue (`|CreateWidget` "/Game/Game/BP/UI/UI_EndScreen.UI_EndScreen_C"))
  (`UserWidget.AddToViewport` _returnvalue 0))

(fn `UserConstructionScript`
  (bind _projectilemovement (`self.ProjectileMovement`))
  (bind _returnvalue (+ (`ProjectileMovementComponent.MaxSpeed` _projectilemovement) (* (`CurveFloat.GetFloatValue` (`self.Speed`) (`GameplayStatics.GetTimeSeconds`)) (`KismetMathLibrary.RandomFloatInRange` 150.0 200.0))))
  (set `ProjectileMovementComponent.MaxSpeed` _returnvalue _projectilemovement)
  (set `ProjectileMovementComponent.InitialSpeed` _returnvalue _projectilemovement))