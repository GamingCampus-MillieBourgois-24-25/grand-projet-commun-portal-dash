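; BP_Spaceship is a player-controlled spaceship that adds the player mapping context on BeginPlay and thrusts upward while IA_Fly is held.
; Each Tick, RotationSpaceship checks IsFlying, applies a physics force along the ship's up vector, and calls RotationUp or RotationDown unless their stop flags are set.
; Both rotation events are empty; the roll-limit logic and a laser spawn with audio sit in unconnected nodes that never run.
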(event `self.ReceiveBeginPlay`
  ;[1 1 1] Récupère IMC
  (bind _asplayer_controller (cast `PlayerController` (`self.GetController`)))
  (bind _returnvalue (pcsubsystem `EnhancedInputLocalPlayerSubsystem` _asplayer_controller))
  (`/Engine/EditorBlueprintResources/StandardMacros.IsValid` _returnvalue
    (:`Is Valid`
      (`EnhancedInputSubsystemInterface.AddMappingContext` _returnvalue "/Game/Game/PlayerInput/IMC_PlayerMouvement.IMC_PlayerMouvement" 1 (struct)))))

(event `self.ReceiveTick`
  (params (DeltaSeconds :type "Float (single-precision)"))
  ;[1 1 1] Tick
  (`self.Rotation Spaceship`))

(event `EnhancedInput|/Game/Game/PlayerInput/Input_Action/IA_Fly`
  (params (ActionValue :type Boolean) (ElapsedSeconds :type "Float (double-precision)") (TriggeredSeconds :type "Float (double-precision)") (InputAction :type "InputAction Object Reference" :default "/Game/Game/PlayerInput/Input_Action/IA_Fly.IA_Fly"))
  ;[1 1 1] Vérif si le joueur clique sur Fly
  (:`Started`
    (set `self.bIsFlying` true :!label _label))
  (:`Ongoing`
    (goto _label))
  (:`Canceled`
    (set `self.bIsFlying` false :!label _label_2)
    (set `self.bStopRotationUp` false)
    (set `self.bStopRotationDown` false)
    (set `self.IsRotationUp` false)
    (set `self.IsRotationDown` false))
  (:`Completed`
    (goto _label_2)))

(event `Rotation Up`
  ;[1 1 1] Rotation Up
)

(event `Add Force Up`
  (bind _spaceship (`self.Spaceship`))
  ;[1 1 1] Force Up Spaceship
  (`PrimitiveComponent.AddForce` _spaceship (* (`SceneComponent.GetUpVector` _spaceship) (`self.fForce`)) "None" false))

(event `Rotation Down`
  ;[1 1 1] Rotation Down
)

(event `Rotation Spaceship`
  ;[1 1 1] Rotation Spaceship
  (if (`self.bIsFlying`)
    (`self.Add Force Up`)
    (if (not (`self.bStopRotationUp`))
      (set `self.IsRotationDown` false)
      (`self.Rotation Up`))
    (elif (not (`self.bStopRotationDown`))
      (set `self.IsRotationUp` false)
      (`self.Rotation Down`))))

(fn `UserConstructionScript`)