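; Shield power-up pickup that grants a BP_Shield to the spaceship, snow player or wagon that touches it.
; On box overlap, it casts for each type, spawns the shield, attaches it to that actor's body component and destroys itself.
; The shield receives snow player and spaceship references, but none for the wagon.
; At BeginPlay, its projectile movement is deactivated if BP_SnowGameManager reports the snow game is playing.
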(event `self.ReceiveBeginPlay`
  (bind _returnvalue (`GameplayStatics.GetActorOfClass` "/Game/Game/BP/Snow/BP_SnowGameManager.BP_SnowGameManager_C"))
  (`/Engine/EditorBlueprintResources/StandardMacros.IsValid` _returnvalue
    (:`Is Valid`
      (if (`/Game/Game/BP/Snow/BP_SnowGameManager.IsSnowPlaying` _returnvalue)
        (`ActorComponent.Deactivate` (`self.ProjectileMovement`))))))

(event `self.Box.OnComponentBeginOverlap`
  (params (OverlappedComponent :type "PrimitiveComponent Object Reference") (OtherActor :type "Actor Object Reference") (OtherComp :type "PrimitiveComponent Object Reference") (OtherBodyIndex :type Integer) (bFromSweep :type Boolean) (SweepResult :type "HitResult Structure (by ref)"))
  (`|ExecutionSequence`
    (:`then_0`
      (bind _asbp_spaceship (cast `/Game/Game/BP/Space/BP_Spaceship` OtherActor))
      (set `self.Parent` (`/Game/Game/BP/Space/BP_Spaceship.Spaceship` _asbp_spaceship)))
    (:`then_1`
      (bind _asbp_snow_player (cast `/Game/Game/BP/Snow/BP_SnowPlayer` OtherActor))
      (set `self.Parent` (`/Game/Game/BP/Snow/BP_SnowPlayer.portaldash_3d_snow_character` _asbp_snow_player)))
    (:`then_2`
      (bind _asbp_wagon (cast `/Game/Game/BP/Western/BP_Wagon` OtherActor))
      (set `self.Parent` (`/Game/Game/BP/Western/BP_Wagon.Body` _asbp_wagon))))
  (bind _returnvalue (`|SpawnActorFromClass` "/Game/Game/BP/PowerUps/BP_Shield.BP_Shield_C" (`self.Spawn Transform_0`) "Undefined" "MultiplyWithRoot" null _asbp_snow_player null _asbp_spaceship null))
  (`self.K2_AttachToComponent` _returnvalue (`self.Parent`) "None" "KeepRelative" "KeepRelative" "KeepRelative" false)
  (`self.K2_DestroyActor`))

(fn `UserConstructionScript`)