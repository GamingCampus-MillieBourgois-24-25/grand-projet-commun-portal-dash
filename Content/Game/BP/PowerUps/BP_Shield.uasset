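; BP_Shield is a temporary shield power-up sized to fit whichever player is in the level: snow character, wagon or spaceship.
; On BeginPlay it finds the player actor and sets its Sphere collision radius from that player's component bounds.
; A looping one-second timer counts Time down and destroys the shield at zero.
; Overlapping a bp_ObstacleSpace also destroys the shield itself; other actor types are ignored.
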(event `self.ReceiveBeginPlay`
  ;[1 1 1] Init bouclier
  (bind _returnvalue (`GameplayStatics.GetActorOfClass` "/Game/Game/BP/Snow/BP_SnowPlayer.BP_SnowPlayer_C"))
  (set `self.Snow` _returnvalue)
  (bind _returnvalue_2 (`GameplayStatics.GetActorOfClass` "/Game/Game/BP/Western/BP_Wagon.BP_Wagon_C"))
  (set `self.Western` _returnvalue_2)
  (bind _returnvalue_3 (`GameplayStatics.GetActorOfClass` "/Game/Game/BP/Space/BP_Spaceship.BP_Spaceship_C"))
  (set `self.Space` _returnvalue_3)
  (`KismetSystemLibrary.K2_SetTimerDelegate` (delegate `Timer`) 1.0 true)
  (if (`KismetSystemLibrary.IsValid` (`self.Snow`))
    (`self.SnowSize`)
    (elif (`KismetSystemLibrary.IsValid` (`self.Western`))
      (`self.WesternSize`)
      (elif (`KismetSystemLibrary.IsValid` (`self.Space`))
        (`self.SpaceSize`)))))

(event `Timer`
  ;[1 1 1] Timer
  (bind _result (`/Engine/EditorBlueprintResources/StandardMacros.DecrementInt` (`self.Time`))
    (:`  `
      (bind _output_get (set `self.Time` _result))
      (if (== _output_get 0)
        (`self.K2_DestroyActor`)))))

(event `SnowSize`
  ;[1 1 1] Size shield for Snow
  (`SphereComponent.SetSphereRadius` (`self.Sphere`) (`.SphereRadius` (`KismetSystemLibrary.GetComponentBounds` (`/Game/Game/BP/Snow/BP_SnowPlayer.portaldash_3d_snow_character` (`self.Snow`)))) true))

(event `WesternSize`
  ;[1 1 1] Size shield for Western
  (`SphereComponent.SetSphereRadius` (`self.Sphere`) (`.SphereRadius` (`KismetSystemLibrary.GetComponentBounds` (`/Game/Game/BP/Western/BP_Wagon.player` (`self.Western`)))) true))

(event `SpaceSize`
  ;[1 1 1] Size shield for Space
  (`SphereComponent.SetSphereRadius` (`self.Sphere`) (`.SphereRadius` (`KismetSystemLibrary.GetComponentBounds` (`/Game/Game/BP/Space/BP_Spaceship.Spaceship` (`self.Space`)))) true))

(event `self.Sphere.OnComponentBeginOverlap`
  (params (OverlappedComponent :type "PrimitiveComponent Object Reference") (OtherActor :type "Actor Object Reference") (OtherComp :type "PrimitiveComponent Object Reference") (OtherBodyIndex :type Integer) (bFromSweep :type Boolean) (SweepResult :type "HitResult Structure (by ref)"))
  ;[1 1 1] Collision Obstacle
  (cast `/Game/Game/BP/Obstacles/bp_ObstacleSpace` OtherActor)
  (`self.K2_DestroyActor`))

(fn `UserConstructionScript`)