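; Dash power-up pickup that flags the player's spaceship as dashing and advances the global distance.
; On BeginPlay it caches the BP_Spaceship and the game instance.
; When the ship overlaps its box, it sets IsDash and adds DistanceDash to DistanceGlobal.
; It then destroys all space obstacles and all dash, laser and shield pickups, including itself.
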(event `self.ReceiveBeginPlay`
  ;[1 1 1] Init Dash
  (bind _returnvalue (`GameplayStatics.GetActorOfClass` "/Game/Game/BP/Space/BP_Spaceship.BP_Spaceship_C"))
  (set `self.SpaceShip` _returnvalue)
  (bind _asbp_game_instance (cast `/Game/Game/BP/bp_GameInstance` (`GameplayStatics.GetGameInstance`)))
  (set `self.As Bp Game Instance` _asbp_game_instance))

(event `self.Box.OnComponentBeginOverlap`
  (params (OverlappedComponent :type "PrimitiveComponent Object Reference") (OtherActor :type "Actor Object Reference") (OtherComp :type "PrimitiveComponent Object Reference") (OtherBodyIndex :type Integer) (bFromSweep :type Boolean) (SweepResult :type "HitResult Structure (by ref)"))
  (bind _spaceship (`self.SpaceShip`))
  (bind _as_bp_game_instance (`self.As Bp Game Instance`))
  ;[1 1 1] Dash
  (if (== OtherActor _spaceship)
    (set `/Game/Game/BP/Space/BP_Spaceship.IsDash` true _spaceship)
    (set `/Game/Game/BP/bp_GameInstance.DistanceGlobal` (+ (`/Game/Game/BP/bp_GameInstance.DistanceGlobal` _as_bp_game_instance) (`self.DistanceDash`)) _as_bp_game_instance)
    (`|ExecutionSequence`
      (:`then_0`
        (bind _outactors (`GameplayStatics.GetAllActorsOfClass` "/Game/Game/BP/Obstacles/bp_ObstacleSpace.bp_ObstacleSpace_C"))
        (`self.K2_DestroyActor` _outactors))
      (:`then_1`
        (bind _outactors_2 (`GameplayStatics.GetAllActorsOfClass` "Bp_Dash_C"))
        (`self.K2_DestroyActor` _outactors_2))
      (:`then_2`
        (bind _outactors_3 (`GameplayStatics.GetAllActorsOfClass` "/Game/Game/BP/PowerUps/BP_RecupLaser.BP_RecupLaser_C"))
        (`self.K2_DestroyActor` _outactors_3))
      (:`then_3`
        (bind _outactors_4 (`GameplayStatics.GetAllActorsOfClass` "/Game/Game/BP/PowerUps/BP_RecupShield.BP_RecupShield_C"))
        (`self.K2_DestroyActor` _outactors_4)))
    (`self.K2_DestroyActor`)))

(fn `UserConstructionScript`)