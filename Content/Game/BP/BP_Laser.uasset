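; BP_Laser is a timed laser actor that follows the player's spaceship and destroys space obstacles it overlaps.
; On BeginPlay it finds BP_Spaceship and starts a looping one-second timer that counts down Time, destroying the laser at zero.
; Each Tick it copies the ship mesh's rotation and snaps to a position offset along that mesh's right vector.
; Its Box overlap destroys any bp_ObstacleSpace it touches.
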(event `self.ReceiveBeginPlay`
  ;[1 1 1] Init Laser
  (bind _returnvalue (`GameplayStatics.GetActorOfClass` "/Game/Game/BP/BP_Spaceship.BP_Spaceship_C"))
  (set `self.SpaceShip` _returnvalue)
  (`KismetSystemLibrary.K2_SetTimerDelegate` (delegate `Timer`) 1.0 true))

(event `Timer`
  ;[1 1 1] Timer
  (bind _result (`/Engine/EditorBlueprintResources/StandardMacros.DecrementInt` (`self.Time`))
    (:`  `
      (bind _output_get (set `self.Time` _result))
      (if (== _output_get 0)
        (`self.K2_DestroyActor`)))))

(event `self.Box.OnComponentBeginOverlap`
  (params (OverlappedComponent :type "PrimitiveComponent Object Reference") (OtherActor :type "Actor Object Reference") (OtherComp :type "PrimitiveComponent Object Reference") (OtherBodyIndex :type Integer) (bFromSweep :type Boolean) (SweepResult :type "HitResult Structure (by ref)"))
  ;[1 1 1] Destroy Obstacle
  (bind _asbp_obstacle_space (cast `/Game/Game/BP/bp_ObstacleSpace` OtherActor))
  (`self.K2_DestroyActor` _asbp_obstacle_space))

(event `self.ReceiveTick`
  (params (DeltaSeconds :type "Float (single-precision)"))
  (bind _spaceship (`/Game/Game/BP/BP_Spaceship.Spaceship` (`self.SpaceShip`)))
  ;[1 1 1] Move which SpaceShip
  (if (`KismetSystemLibrary.IsValid` (`self.SpaceShip`))
    (`self.K2_SetActorLocation` (+ (`SceneComponent.K2_GetComponentLocation` _spaceship) (* (`SceneComponent.GetRightVector` _spaceship) 75.0)))
    (`self.K2_SetActorRotation` (`SceneComponent.K2_GetComponentRotation` (`/Game/Game/BP/BP_Spaceship.Spaceship` (`self.SpaceShip`))))))

(fn `UserConstructionScript`)