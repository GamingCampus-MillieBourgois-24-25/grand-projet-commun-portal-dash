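; BP_WesternManager is a spawner that, from BeginPlay, endlessly spawns coin or lasso actors at its own transform.
; Its SpawnObstacle event picks a random branch, waits a fixed short delay, spawns the actor, then calls itself to repeat.
; Two of the three branches spawn BP_Coin and one spawns BP_Lasso, weighting the odds toward coins.
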(event `self.ReceiveBeginPlay`
  (`self.SpawnObstacle`))

(event `SpawnObstacle`
  (switch `int` (`KismetMathLibrary.RandomInteger` 3)
    (:`0`
      (`KismetSystemLibrary.Delay` 2.0)
      (`|SpawnActorFromClass` "/Game/Game/BP/BP_Coin.BP_Coin_C" (`self.GetTransform`) "Undefined" "MultiplyWithRoot" null null)
      (`self.SpawnObstacle`))
    (:`1`
      (`KismetSystemLibrary.Delay` 2.0)
      (`|SpawnActorFromClass` "/Game/Game/BP/BP_Coin.BP_Coin_C" (`self.GetTransform`) "Undefined" "MultiplyWithRoot" null null)
      (`self.SpawnObstacle`))
    (:`2`
      (`KismetSystemLibrary.Delay` 2.0)
      (`|SpawnActorFromClass` "/Game/Game/BP/BP_Lasso.BP_Lasso_C" (`self.GetTransform`) "Undefined" "MultiplyWithRoot" null null)
      (`self.SpawnObstacle`))))

(fn `UserConstructionScript`)