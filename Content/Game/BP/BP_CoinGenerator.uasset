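; Spawner actor that keeps generating coin or lasso pickups (BP_Coin, BP_Lasso) at three spawn points, faster as game time passes.
; Tick rerolls a random selector that SpawnObstacle reads to pick one spawner or a pair.
; Each spawner waits on a Delay shrinking with game time up to MaxTime, spawns either class at random, then calls SpawnObstacle again to loop.
; The random start value set on BeginPlay is never read.
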(event `self.ReceiveBeginPlay`
  ;[1 1 1] Call Obstacle on BeginPlay
  (set `self.FRandomBegin` (`KismetMathLibrary.RandomFloatInRange` 3.0 6.0))
  (`KismetSystemLibrary.Delay` 0.2)
  (`self.Spawn Obstacle`))

(event `Spawn Obstacle`
  (bind _returnvalue (`KismetMathLibrary.RandomInteger` 2))
  (bind _ispawneractivate (`self.iSpawnerActivate`))
  (bind _returnvalue_2 (`SceneComponent.K2_GetComponentToWorld` (`self.Spawner1`)))
  (bind _returnvalue_3 (`SceneComponent.K2_GetComponentToWorld` (`self.Spawner2`)))
  (bind _returnvalue_4 (`KismetMathLibrary.MapRangeClamped` (`KismetSystemLibrary.GetGameTimeInSeconds`) 0.0 (`self.MaxTime`) 3.0 1.0))
  (bind _returnvalue_5 (`SceneComponent.K2_GetComponentToWorld` (`self.Spawner`)))
  ;[1 1 1] Spawn Obstacle with Delay that decreased with the time
  (if (< _ispawneractivate 4)
    (`KismetSystemLibrary.Delay` _returnvalue_4 :!label _label)
    (switch `int` _returnvalue
      (:`0`
        (`|SpawnActorFromClass` "/Game/Game/BP/BP_Coin.BP_Coin_C" _returnvalue_5 "Undefined" "MultiplyWithRoot" null null))
      (:`1`
        (`|SpawnActorFromClass` "/Game/Game/BP/BP_Lasso.BP_Lasso_C" _returnvalue_5 "Undefined" "MultiplyWithRoot" null null)))
    (elif (< _ispawneractivate 7)
      (`KismetSystemLibrary.Delay` _returnvalue_4 :!label _label_2)
      (switch `int` _returnvalue
        (:`0`
          (`|SpawnActorFromClass` "/Game/Game/BP/BP_Coin.BP_Coin_C" _returnvalue_2 "Undefined" "MultiplyWithRoot" null null))
        (:`1`
          (`|SpawnActorFromClass` "/Game/Game/BP/BP_Lasso.BP_Lasso_C" _returnvalue_2 "Undefined" "MultiplyWithRoot" null null)))
      (else
        (if (< _ispawneractivate 10)
          _
          (elif (== _ispawneractivate 10)
            (`|ExecutionSequence`
              (:`then_0`
                (goto _label))
              (:`then_1`
                (goto _label_2)))
            (elif (== _ispawneractivate 11)
              (`|ExecutionSequence`
                (:`then_0`
                  (goto _label_2))
                (:`then_1`
                  _))
              (else
                (`|ExecutionSequence`
                  (:`then_0`
                    (goto _label))
                  (:`then_1`
                    _))))))
        (`KismetSystemLibrary.Delay` _returnvalue_4)
        (switch `int` _returnvalue
          (:`0`
            (`|SpawnActorFromClass` "/Game/Game/BP/BP_Coin.BP_Coin_C" _returnvalue_3 "Undefined" "MultiplyWithRoot" null null))
          (:`1`
            (`|SpawnActorFromClass` "/Game/Game/BP/BP_Lasso.BP_Lasso_C" _returnvalue_3 "Undefined" "MultiplyWithRoot" null null))))))
  (`self.Spawn Obstacle`))

(event `self.ReceiveTick`
  (params (DeltaSeconds :type "Float (single-precision)"))
  ;[1 1 1] Set wich spawner activate
  (set `self.iSpawnerActivate` (`KismetMathLibrary.RandomIntegerInRange` 1 12)))

(fn `UserConstructionScript`)