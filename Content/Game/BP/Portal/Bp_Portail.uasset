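; Portal actor that ends the current space level and switches worlds when the BP_Spaceship enters its box.
; On overlap it destroys the ground generator, ground segments, obstacle manager, slide-scrolling actor and spaceship, and has the game instance clear obstacles.
; It then gives itself a short lifespan and calls ChangeWorld on the game instance.
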(event `self.Box.OnComponentBeginOverlap`
  (params (OverlappedComponent :type "PrimitiveComponent Object Reference") (OtherActor :type "Actor Object Reference") (OtherComp :type "PrimitiveComponent Object Reference") (OtherBodyIndex :type Integer) (bFromSweep :type Boolean) (SweepResult :type "HitResult Structure (by ref)"))
  (cast `/Game/Game/BP/Space/BP_Spaceship` OtherActor)
  (`KismetSystemLibrary.PrintString` "portal")
  (`|ExecutionSequence`
    (:`then_0`
      (bind _returnvalue (`GameplayStatics.GetActorOfClass` "/Game/Game/BP/Space/BP_GroundGenerator.BP_GroundGenerator_C"))
      (`self.K2_DestroyActor` _returnvalue))
    (:`then_1`
      (bind _outactors (`GameplayStatics.GetAllActorsOfClass` "/Game/Game/BP/Space/BP_Ground1SpaceLevel.BP_Ground1SpaceLevel_C"))
      (`self.K2_DestroyActor` _outactors)
      (bind _outactors_2 (`GameplayStatics.GetAllActorsOfClass` "/Game/Game/BP/Space/BP_Ground2SpaceLevel.BP_Ground2SpaceLevel_C"))
      (`self.K2_DestroyActor` _outactors_2)
      (bind _outactors_3 (`GameplayStatics.GetAllActorsOfClass` "/Game/Game/BP/Space/BP_Ground3SpaceLevel.BP_Ground3SpaceLevel_C"))
      (`self.K2_DestroyActor` _outactors_3))
    (:`then_2`
      (bind _returnvalue_2 (`GameplayStatics.GetActorOfClass` "/Game/Game/BP/Obstacles/Bp_ObstacleManager.Bp_ObstacleManager_C"))
      (`self.K2_DestroyActor` _returnvalue_2))
    (:`then_3`
      (bind _asbp_game_instance (cast `/Game/Game/BP/bp_GameInstance` (`GameplayStatics.GetGameInstance`)))
      (`/Game/Game/BP/bp_GameInstance.destroyObstacle` _asbp_game_instance))
    (:`then_4`
      (bind _returnvalue_3 (`GameplayStatics.GetActorOfClass` "/Game/Game/BP/Space/BP_Slide_scrolling.BP_Slide_scrolling_C"))
      (`self.K2_DestroyActor` _returnvalue_3))
    (:`then_5`
      (bind _returnvalue_4 (`GameplayStatics.GetActorOfClass` "/Game/Game/BP/Space/BP_Spaceship.BP_Spaceship_C"))
      (`self.K2_DestroyActor` _returnvalue_4)
      (`self.SetLifeSpan` 3.0)
      (`/Game/Game/BP/bp_GameInstance.ChangeWorld` _asbp_game_instance))))

(fn `UserConstructionScript`)