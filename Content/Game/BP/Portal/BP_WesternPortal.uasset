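; BP_WesternPortal is the exit portal of the Western level, tearing that world down and switching worlds when the wagon reaches it.
; A box overlap by BP_Wagon runs a sequence that destroys Western actors by class lookup, including wagon, manager, generators, rails, obstacles, pickups and lassos.
; Midway through, it also destroys the first portal found, then calls ChangeWorld on the game instance before finishing the remaining cleanup.
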(event `self.Box.OnComponentBeginOverlap`
  (params (OverlappedComponent :type "PrimitiveComponent Object Reference") (OtherActor :type "Actor Object Reference") (OtherComp :type "PrimitiveComponent Object Reference") (OtherBodyIndex :type Integer) (bFromSweep :type Boolean) (SweepResult :type "HitResult Structure (by ref)"))
  (cast `/Game/Game/BP/Western/BP_Wagon` OtherActor)
  (`self.SetLifeSpan` 2.0)
  (`KismetSystemLibrary.PrintString` "portal")
  (`|ExecutionSequence`
    (:`then_0`
      (bind _outactors (`GameplayStatics.GetAllActorsOfClass` "/Game/Game/BP/Western/BP_Wagon.BP_Wagon_C"))
      (`self.K2_DestroyActor` _outactors))
    (:`then_1`
      (bind _outactors_2 (`GameplayStatics.GetAllActorsOfClass` "/Game/Game/BP/Western/BP_RailGeneratorLevelWestern.BP_RailGeneratorLevelWestern_C"))
      (`self.K2_DestroyActor` _outactors_2))
    (:`then_2`
      (bind _outactors_3 (`GameplayStatics.GetAllActorsOfClass` "/Game/Game/BP/Western/BP_WesternManager.BP_WesternManager_C"))
      (`self.K2_DestroyActor` _outactors_3))
    (:`then_3`
      (bind _outactors_4 (`GameplayStatics.GetAllActorsOfClass` "/Game/Game/BP/Obstacles/BP_ObstableGeneratorWesternLevel.BP_ObstableGeneratorWesternLevel_C"))
      (`self.K2_DestroyActor` _outactors_4))
    (:`then_4`
      (bind _outactors_5 (`GameplayStatics.GetAllActorsOfClass` "/Game/Game/BP/Western/BP_Rail_Western.BP_Rail_Western_C"))
      (`self.K2_DestroyActor` _outactors_5))
    (:`then_5`
      (bind _outactors_6 (`GameplayStatics.GetAllActorsOfClass` "/Game/Game/BP/Obstacles/bp_ObstacleWestern.bp_ObstacleWestern_C"))
      (`self.K2_DestroyActor` _outactors_6))
    (:`then_6`
      (bind _returnvalue (`GameplayStatics.GetActorOfClass` "BP_WesternPortal_C"))
      (`self.K2_DestroyActor` _returnvalue))
    (:`then_7`
      (`self.SetLifeSpan` 3.0)
      (bind _asbp_game_instance (cast `/Game/Game/BP/bp_GameInstance` (`GameplayStatics.GetGameInstance`)))
      (`/Game/Game/BP/bp_GameInstance.ChangeWorld` _asbp_game_instance))
    (:`then_8`
      (bind _outactors_7 (`GameplayStatics.GetAllActorsOfClass` "/Game/Game/BP/PowerUps/BP_Lasso.BP_Lasso_C"))
      (`self.K2_DestroyActor` _outactors_7))
    (:`then_9`
      (bind _outactors_8 (`GameplayStatics.GetAllActorsOfClass` "/Game/Game/BP/PowerUps/BP_Coin.BP_Coin_C"))
      (`self.K2_DestroyActor` _outactors_8))
    (:`then_10`
      (bind _outactors_9 (`GameplayStatics.GetAllActorsOfClass` "/Game/Game/BP/PowerUps/BP_TNTobject.BP_TNTobject_C"))
      (`self.K2_DestroyActor` _outactors_9))
    (:`then_11`
      (bind _outactors_10 (`GameplayStatics.GetAllActorsOfClass` "/Game/Game/BP/Western/BP_GroundStartWesternLevel.BP_GroundStartWesternLevel_C"))
      (`self.K2_DestroyActor` _outactors_10))
    (:`then_12`
      (bind _returnvalue_2 (`GameplayStatics.GetActorOfClass` "/Game/Game/BP/PowerUps/BP_ActiveLasso.BP_ActiveLasso_C"))
      (`self.K2_DestroyActor` _returnvalue_2))))

(fn `UserConstructionScript`)