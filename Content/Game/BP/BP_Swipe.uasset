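; BP_Swipe detects touch swipes and classifies them as up, down, left or right.
; Touch press stores the start point and enables a per-tick check; release stores the end point and resets a DoOnce.
; The check compares start to the stored end against a distance threshold, then samples the live touch once and picks the dominant axis.
; Vertical swipes set GoUp or GoDown; horizontal ones only print, and IsPressed is never cleared.
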(event `self.ReceiveTick`
  (params (DeltaSeconds :type "Float (single-precision)"))
  (if (`self.Is Pressed`)
    (`self.Check_Swiping`)))

(event `Check_Swiping`
  (bind (_locationx _locationy) (`self.GetInputTouchState` (`GameplayStatics.GetPlayerController` 0) "Touch1"))
  (bind (_x _y) (`KismetMathLibrary.BreakVector2D` (- (`self.TouchStart`) (`self.TouchEnd`))))
  (if (> (`KismetMathLibrary.VSize2D` (- (`self.TouchStart`) (`self.TouchEnd`))) 100.0)
    (`/Engine/EditorBlueprintResources/StandardMacros.DoOnce` false :!label _label
      (:`Completed`
        (set `self.TouchEnd` (`KismetMathLibrary.MakeVector2D` _locationx _locationy))
        (if (> (`KismetMathLibrary.Abs` _x) (`KismetMathLibrary.Abs` _y))
          (if (> _x 0.0)
            (`KismetSystemLibrary.PrintString` "left")
            (else
              (`KismetSystemLibrary.PrintString` "right")))
          (elif (> _y 0.0)
            (`|ExecutionSequence`
              (:`then_0`
                (set `self.GoUp` true))
              (:`then_1`
                (`KismetSystemLibrary.PrintString` "up")))
            (else
              (`|ExecutionSequence`
                (:`then_0`
                  (set `self.GoDown` true))
                (:`then_1`
                  (`KismetSystemLibrary.PrintString` "down"))))))))))

(event `InputTouch`
  (params (Location :type "Vector Structure") (FingerIndex :type "ETouchIndex Enum"))
  (bind _x (.x Location))
  (bind _y (.y Location))
  (:`Pressed`
    (set `self.Is Pressed` true)
    (set `self.TouchStart` (`KismetMathLibrary.MakeVector2D` _x _y)))
  (:`Released`
    (set `self.TouchEnd` (`KismetMathLibrary.MakeVector2D` _x _y))
    (goto _label :!via `Reset`)))

(fn `UserConstructionScript`)