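; BP_Wagon is a player-controlled wagon that switches between three lanes with the Left and Right keys, and it creates the BP_UIGame HUD on BeginPlay.
; Each key press computes a clamped target lane and restarts a shared timeline, whose separate Y and Z tracks interpolate the position between per-lane offsets while keeping the mesh's X.
; The current lane updates when the timeline finishes, and both keys also print a debug "Hello".
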(event `self.ReceiveBeginPlay`
  (bind _returnvalue (`|CreateWidget` "/Game/Game/BP/BP_UIGame.BP_UIGame_C"))
  (`UserWidget.AddToViewport` _returnvalue 0))

(event `Key|Left`
  (params (Key :type "Key Structure"))
  (bind _lane_y (`self.Lane Y`))
  (bind _lane_z (`self.Lane Z`))
  (bind _returnvalue_x (`KismetMathLibrary.BreakVector` (`SceneComponent.K2_GetComponentLocation` (`self.StaticMesh`))))
  (:`Pressed`
    (`|ExecutionSequence`
      (:`then_0`
        (set `self.NewLane` (`KismetMathLibrary.Clamp` (+ (`self.Lane`) -1) 0 2))
        (bind (_direction _lane_y_2 _lane_z_2) (`Timeline|Chronologie` :!via `PlayFromStart` :!label _label)
          (:`Update`
            (`self.K2_SetActorLocation` (`KismetMathLibrary.MakeVector` _returnvalue_x (`KismetMathLibrary.Lerp` (`|GetArrayItem` _lane_y (`self.Lane`)) (`|GetArrayItem` _lane_y (`self.NewLane`)) _lane_y_2) (`KismetMathLibrary.Lerp` (`|GetArrayItem` _lane_z (`self.Lane`)) (`|GetArrayItem` _lane_z (`self.NewLane`)) _lane_z_2))))
          (:`Finished`
            (set `self.Lane` (`self.NewLane`)))))
      (:`then_1`
        (`KismetSystemLibrary.PrintString` "Hello")))))

(event `Key|Right`
  (params (Key :type "Key Structure"))
  (:`Pressed`
    (`|ExecutionSequence`
      (:`then_0`
        (set `self.NewLane` (`KismetMathLibrary.Clamp` (+ (`self.Lane`) 1) 0 2))
        (goto _label :!via `PlayFromStart`))
      (:`then_1`
        (`KismetSystemLibrary.PrintString` "Hello")))))

(fn `UserConstructionScript`)