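; Physics-driven snow player pawn with Enhanced Input, a variable-height jump and a timed collectible glider.
; Holding the jump input applies force briefly when grounded; component hits set grounded and a downward trace clears it.
; After the jump input is released, holding glide while airborne shows the glider and adds thrust whenever the pawn is not rising.
; Tick drains the glider timer and nudges Y velocity into a set band while grounded or gliding.
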(event `self.ReceiveBeginPlay`
  ;[1 1 1] Get MappingContext
  (bind _asplayer_controller (cast `PlayerController` (`self.GetController`)))
  (bind _returnvalue (pcsubsystem `EnhancedInputLocalPlayerSubsystem` _asplayer_controller))
  (`/Engine/EditorBlueprintResources/StandardMacros.IsValid` _returnvalue
    (:`Is Valid`
      (`EnhancedInputSubsystemInterface.AddMappingContext` _returnvalue "/Game/Game/PlayerInput/IMC_PlayerMouvement.IMC_PlayerMouvement" 1 (struct)))))

(event `EnhancedInput|/Game/Game/PlayerInput/Input_Action/IA_Slider`
  (params (ActionValue :type Boolean) (ElapsedSeconds :type "Float (double-precision)") (TriggeredSeconds :type "Float (double-precision)") (InputAction :type "InputAction Object Reference" :default "/Game/Game/PlayerInput/Input_Action/IA_Slider.IA_Slider"))
  ;[1 1 1] Jump Depending of time pressed
  (:`Ongoing`
    (`|ExecutionSequence`
      (:`then_0`
        (if (> 0.4 ElapsedSeconds)
          (if (stale _output_get)
            (`PrimitiveComponent.AddForce` (`self.portaldash_3d_snow_character`) (`self.Impulse Force`) "None" true))
          (else
            (bind _output_get (set `self.IsJumping` false)))))
      (:`then_1`
        (`/Engine/EditorBlueprintResources/StandardMacros.DoOnce` false :!label _label
          (:`Completed`
            (if (`self.isGrouded`)
              (set `self.IsJumping` true)
              (else
                (set `self.IsJumping` false))))))))
  (:`Canceled`
    (set `self.IsJumping` false :!label _label_2)
    (set `self.CanGlide` true)
    (goto _label :!via `Reset`))
  (:`Completed`
    (goto _label_2)))

(event `self.ReceiveTick`
  (params (DeltaSeconds :type "Float (single-precision)"))
  ;[1 1 1] Tick
  (`self.Ground Check`)
  (`|ExecutionSequence`
    (:`then_0`
      (if (`self.HasGlider`)
        (`self.GliderTick`)))
    (:`then_1`
      (if (or (`self.isGrouded`) (`self.IsGliding`))
        (`self.SpeedTick`)))))

(event `Ground Check`
  (bind _portaldash_3d_snow_character (`self.portaldash_3d_snow_character`))
  (bind _returnvalue (`SceneComponent.K2_GetComponentLocation` _portaldash_3d_snow_character))
  ;[1 1 1] Raycast for leaving the ground
  (bind (_outhit _returnvalue_2) (`KismetSystemLibrary.LineTraceSingle` :`Start` _returnvalue :`End` (+ _returnvalue (* (`self.RayLenght`) (* (`KismetMathLibrary.GetUpVector` (`SceneComponent.K2_GetComponentRotation` _portaldash_3d_snow_character)) -1.0))) :`TraceChannel` "TraceTypeQuery1" :`DrawDebugType` "ForOneFrame"))
  (if (not _returnvalue_2)
    (set `self.isGrouded` false)))

(event `self.portaldash_3d_snow_character.OnComponentHit`
  (params (HitComponent :type "PrimitiveComponent Object Reference") (OtherActor :type "Actor Object Reference") (OtherComp :type "PrimitiveComponent Object Reference") (NormalImpulse :type "Vector Structure") (Hit :type "HitResult Structure (by ref)"))
  ;[1 1 1] Ground Check
  (bind _output_get (set `self.isGrouded` true))
  (if _output_get
    (set `self.CanGlide` false)
    (`KismetSystemLibrary.PrintText` "Grounded" true true (struct :`G` 0.66 :`B` 1.0 :`A` 1.0) 0.1)))

(event `EnhancedInput|/Game/Game/PlayerInput/Input_Action/IA_Glider`
  (params (ActionValue :type Boolean) (ElapsedSeconds :type "Float (double-precision)") (TriggeredSeconds :type "Float (double-precision)") (InputAction :type "InputAction Object Reference" :default "/Game/Game/PlayerInput/Input_Action/IA_Glider.IA_Glider"))
  (bind _portaldash_3d_snow_character (`self.portaldash_3d_snow_character`))
  (bind _returnvalue (`SceneComponent.GetComponentVelocity` _portaldash_3d_snow_character))
  ;[1 1 1] Glider Logic
  (:`Ongoing`
    (if (`self.HasGlider`)
      (if (`self.isGrouded`)
        _
        (elif (`self.CanGlide`)
          (if (not (`self.IsJumping`))
            (bind _output_get (set `self.IsGliding` true))
            (`SceneComponent.SetVisibility` (`self.portaldash_3d_snow_glider`) _output_get false)
            (if (<= (`KismetMathLibrary.Dot_VectorVector` (`KismetMathLibrary.Normal` _returnvalue 0.1) (`SceneComponent.GetUpVector` _portaldash_3d_snow_character)) 0.0)
              (`KismetSystemLibrary.PrintText` (`KismetTextLibrary.Conv_VectorToText` _returnvalue) true true (struct :`G` 0.66 :`B` 1.0 :`A` 1.0) 0.1)
              (`PrimitiveComponent.AddForce` (`self.portaldash_3d_snow_character`) (`self.GliderThrust`) "None" true)))))))
  (:`Canceled`
    (bind _output_get_2 (set `self.IsGliding` false :!label _label_3))
    (`SceneComponent.SetVisibility` (`self.portaldash_3d_snow_glider`) _output_get_2 false))
  (:`Completed`
    (goto _label_3)))

(event `GliderCollected`
  ;[1 1 1] Glider Colection
  (set `self.HasGlider` true)
  (set `self.CurrentGliderTimer` (`self.GliderTimer`))
  (set `self.Glider Reset` false))

(event `SpeedTick`
  (bind _portaldash_3d_snow_character (`self.portaldash_3d_snow_character`))
  (bind _y (.y (`self.GetVelocity`)))
  (bind _returnvalue (or (`self.isGrouded`) (`self.IsGliding`)))
  ;[1 1 1] PlayerSpeedCheck
  (`KismetSystemLibrary.PrintText` (`KismetTextLibrary.Conv_DoubleToText` _y "HalfToEven") true true (struct :`G` 0.66 :`B` 1.0 :`A` 1.0) 0.1)
  (`|ExecutionSequence`
    (:`then_0`
      (if (and (> _y 2600.0) _returnvalue)
        (`KismetSystemLibrary.PrintString` "Fast" true true (struct :`R` 1.0 :`A` 1.0) 0.1)
        (`PrimitiveComponent.SetPhysicsLinearVelocity` _portaldash_3d_snow_character (0.0 -20.0 0.0) true "None")))
    (:`then_1`
      (if (and (< _y 700.0) _returnvalue)
        (`KismetSystemLibrary.PrintString` "Slow" true true (struct :`R` 1.0 :`G` 0.090447 :`A` 1.0) 0.1)
        (`PrimitiveComponent.SetPhysicsLinearVelocity` _portaldash_3d_snow_character (0.0 20.0 0.0) true "None")))))

(event `GliderTick`
  ;[1 1 1] Glider Tick
  (set `self.CurrentGliderTimer` (`KismetMathLibrary.FClamp` (- (`self.CurrentGliderTimer`) (`GameplayStatics.GetWorldDeltaSeconds`)) 0.0 (`self.CurrentGliderTimer`)))
  (if (<= (`self.CurrentGliderTimer`) 0.0)
    (set `self.HasGlider` false)))

(fn `UserConstructionScript`)