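; Procedural snow terrain chunk that builds a randomized slope from a spline, with gaps and spawned gameplay actors.
; BeginPlay draws the spline, adding a gentler incline on level start and recording crests, then lays random spline meshes with holes possible at or just after crests.
; A final pass scatters coins, shield pickups and obstacles using cooldown and hole-clearance checks.
; It stores end and three-quarter positions, and a separate event spawns a portal.
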(event `Obstacle Generation`
  (bind _splinestart (`self.SplineStart`))
  (bind _currentindex (`self.CurrentIndex`))
  (bind _ishole (`self.IsHole`))
  (bind _returnvalue (`KismetMathLibrary.MakeTransform` (+ (.location (`SplineComponent.GetTransformAtSplinePoint` (`self.TerrainSpline`) (`self.CurrentIndex`) "World" false)) (0.0 0.0 100.0)) (.rotation (`SplineComponent.GetTransformAtSplinePoint` (`self.TerrainSpline`) (`self.CurrentIndex`) "World" false)) (.scale (`SplineComponent.GetTransformAtSplinePoint` (`self.TerrainSpline`) (`self.CurrentIndex`) "World" false))))
  (for _index (range 3 (`SplineComponent.GetNumberOfSplinePoints` (`self.TerrainSpline`)))
    (bind _output_get (set `self.CurrentIndex` _index))
    (`|ExecutionSequence`
      (:`then_0`
        (if (and _splinestart (== _output_get 25))
          (set `self.SplineStart` false)))
      (:`then_1`
        (if _splinestart
          (if (> (`KismetMathLibrary.RandomIntegerInRange` 0 100) 70)
            (bind _returnvalue_2 (`|SpawnActorFromClass` "/Game/Game/BP/PowerUps/BP_Coin.BP_Coin_C" (`KismetMathLibrary.MakeTransform` (+ (.location _returnvalue) (0.0 0.0 100.0)) (.rotation _returnvalue) (.scale _returnvalue)) "Undefined" "MultiplyWithRoot" null null :!label _label))
            (`self.SetActorScale3D` _returnvalue_2 (3.0 3.0 3.0)))
          (else
            (`|ExecutionSequence`
              (:`then_0`
                (if (!= (`self.CanGenerate`) 0)
                  (`/Engine/EditorBlueprintResources/StandardMacros.DecrementInt` (`self.CanGenerate`))))
              (:`then_1`
                (if (and (not (`|GetArrayItem` (`self.IsHole`) (`self.CurrentIndex`))) (== (`self.CanGenerate`) 0))
                  (switch `int` (`KismetMathLibrary.RandomIntegerInRange` 0 1)
                    (:`Default`
                      _)
                    (:`0`
                      (goto _label))
                    (:`1`
                      _))
                  (if (not (or (`|GetArrayItem` _ishole (+ _currentindex 1)) (`|GetArrayItem` _ishole (+ _currentindex 2)) (`|GetArrayItem` _ishole (- _currentindex 1)) (`|GetArrayItem` _ishole (- _currentindex 2))))
                    (if (> (`KismetMathLibrary.RandomIntegerInRange` 0 100) 30)
                      (`KismetArrayLibrary.Array_Set` (`self.HasObstacle`) (`self.CurrentIndex`) true)
                      (set `self.CanGenerate` 4)
                      (if (> (`KismetMathLibrary.RandomIntegerInRange` 0 100) 70)
                        (`/Engine/EditorBlueprintResources/StandardMacros.FlipFlop`
                          (:`A`
                            (switch `int` (`KismetMathLibrary.RandomIntegerInRange` 0 2)
                              (:`0`
                                _)
                              (:`1`
                                _)
                              (:`2`
                                _))
                            (bind _returnvalue_3 (`|SpawnActorFromClass` "/Game/Game/BP/PowerUps/BP_RecupShield.BP_RecupShield_C" (`KismetMathLibrary.MakeTransform` (+ (.location _returnvalue) (0.0 0.0 100.0)) (.rotation _returnvalue) (2.0 2.0 2.0)) "Undefined" "MultiplyWithRoot" null null))
                            (`self.SetLifeSpan` _returnvalue_3 60.0))
                          (:`B`
                            (bind _returnvalue_4 (`|SpawnActorFromClass` "/Game/Game/BP/Obstacles/BP_SnowObstacle.BP_SnowObstacle_C" _returnvalue "Undefined" "MultiplyWithRoot" null null :!label _label_2))
                            (`self.SetLifeSpan` _returnvalue_4 60.0)))
                        (else
                          (goto _label_2))))))))))))))

(event `GeneratePortal`
  (`KismetSystemLibrary.PrintText` "Generated Portal" true true (struct :`R` 1.0 :`B` 0.367797 :`A` 1.0) 60.0)
  (`|SpawnActorFromClass` "/Game/Game/BP/Portal/Bp_SnowPortal.Bp_SnowPortal_C" (`KismetMathLibrary.MakeTransform` (+ (.location (`SplineComponent.GetTransformAtSplinePoint` (`self.TerrainSpline`) 27 "World" false)) (0.0 0.0 500.0)) (struct) (.scale (`SplineComponent.GetTransformAtSplinePoint` (`self.TerrainSpline`) 27 "World" false))) "Undefined" "MultiplyWithRoot" null null))

(event `Generate Mesh`
  (bind _returnvalue (- (`SplineComponent.GetNumberOfSplinePoints` (`self.TerrainSpline`)) 1))
  ;[1 0.01528 0] Mesh Creation
  ;;[1 1 1] Loop for Mesh Generation
  (`|ExecutionSequence`
    (:`then_0`
      (`/Engine/EditorBlueprintResources/StandardMacros.DoOnce` false
        (:`Completed`
          (`KismetArrayLibrary.Array_Resize` (`self.IsHole`) _returnvalue)
          (`KismetArrayLibrary.Array_Resize` (`self.HasObstacle`) _returnvalue))))
    (:`then_1`
      (for _index (range 3 (+ _returnvalue 1))
        (bind _output_get (set `self.CurrentIndex` _index))
        (if (and (`self.SplineStart`) (< _output_get (`self.StartInclineLenght`)))
          (`self.AddMesh`)
          (else
            (`self.HoleLogic`))))
      (`self.Obstacle Generation`))))

(event `AddMesh`
  (bind _currentindex (`self.CurrentIndex`))
  (bind _terrainspline (`self.TerrainSpline`))
  (bind (_location _tangent) (`SplineComponent.GetLocationAndTangentAtSplinePoint` _terrainspline _currentindex "Local"))
  (bind (_location_2 _tangent_2) (`SplineComponent.GetLocationAndTangentAtSplinePoint` _terrainspline (- _currentindex 1) "Local"))
  ;[1 0.01528 0] Mesh Creation
  ;;[1 1 1] Add mesh to the spline point when called
  (bind _returnvalue (`AddComponent|NODE_AddSplineMeshComponent-0`))
  (`StaticMeshComponent.SetStaticMesh` _returnvalue (`KismetArrayLibrary.Array_Random` (`self.GroundMesh`)))
  (`SceneComponent.K2_AttachToComponent` _returnvalue null "None" "KeepRelative" "KeepRelative" "KeepRelative" true)
  (`SplineMeshComponent.SetStartAndEnd` _returnvalue _location_2 _tangent_2 _location _tangent true)
  (`PrimitiveComponent.SetMaterial` (`self.TerrainSpline`) 0 "/Game/Game/asset/Snow_Assets/Ground/sha_sol_snow.sha_sol_snow")
  (`PrimitiveComponent.SetCollisionEnabled` _returnvalue "QueryAndPhysics"))

(event `HoleLogic`
  (bind _splineup (`self.SplineUp`))
  (bind _currentindex (`self.CurrentIndex`))
  ;[1 0.01528 0] Mesh Creation
  ;;[1 1 1] Hole Logic
  ;;;[1 1 1] Has an 70% chance of generating a hole
  (if (`KismetMathLibrary.BooleanNOR` (`KismetArrayLibrary.Array_Contains` _splineup _currentindex) (or (and (`KismetArrayLibrary.Array_Contains` _splineup (- _currentindex 1)) (> (`KismetMathLibrary.RandomIntegerInRange` 0 100) 40)) (and (`KismetArrayLibrary.Array_Contains` _splineup (- _currentindex 2)) (> (`KismetMathLibrary.RandomIntegerInRange` 0 100) 80))))
    (`self.AddMesh` :!label _label_3)
    (elif (> (`KismetMathLibrary.RandomIntegerInRange` 0 100) 30)
      (goto _label_3)
      (else
        (`KismetArrayLibrary.Array_Set` (`self.IsHole`) (`self.CurrentIndex`) true)))))

(event `LastPos`
  (bind _terrainspline (`self.TerrainSpline`))
  (bind _returnvalue (`SplineComponent.GetNumberOfSplinePoints` _terrainspline))
  ;[0 0.09973 0.1094] Generate Spline
  ;;[1 1 1] Get the last spline point pos
  (set `self.SplineLastPos` (`SplineComponent.GetLocationAtSplinePoint` _terrainspline (- _returnvalue 1) "World"))
  (set `self.3/4 Mark` (`SplineComponent.GetLocationAtSplinePoint` _terrainspline (* (/ _returnvalue 4) 3) "World")))

(event `self.ReceiveBeginPlay`
  (bind _terrainspline (`self.TerrainSpline`))
  ;[0 0.09973 0.1094] Generate Spline
  ;;[1 1 1] Clear + Start Spline
  (`SplineComponent.ClearSplinePoints` _terrainspline true)
  (`SplineComponent.AddSplinePoint` _terrainspline (`self.StartPosition`) "Local" true)
  (`SplineComponent.AddSplinePointAtIndex` _terrainspline (`KismetMathLibrary.CreateVectorFromYawPitch` -90.0 (`KismetMathLibrary.RandomFloatInRange` -5.0 -30.0) 600.0) 0 "Local" true)
  (set `self.SplineInitialPos` (`SceneComponent.K2_GetComponentLocation` (`self.DefaultSceneRoot`)))
  (bind _returnvalue (`GameplayStatics.GetActorOfClass` "/Game/Game/BP/Snow/BP_SnowGameManager.BP_SnowGameManager_C"))
  (set `self.LevelStart` (`/Game/Game/BP/Snow/BP_SnowGameManager.IsStart` _returnvalue))
  (set `self.SplineStart` false)
  (`self.DrawLine`))

(event `NormalSpline`
  (params (SplineLocation :type "Vector Structure") (SplineRotation :type "Vector Structure") (`SplinePoint ` :type Integer))
  ;[0 0.09973 0.1094] Generate Spline
  ;;[1 1 1] Add New Spline After Start
  (bind _result (`/Engine/EditorBlueprintResources/StandardMacros.IncrementInt` `SplinePoint `)
    (:`  `
      (`SplineComponent.AddSplinePoint` (`self.TerrainSpline`) (+ SplineLocation SplineRotation) "Local" true)
      (if (< `SplinePoint ` (`self.TotalSplineInOne`))
        (if true
          (`self.IsSplineGoingUp?`)
          (if (`self.IsSplineGoingUp`)
            (`KismetArrayLibrary.Array_Add` (`self.SplineUp`) _result)))))))

(event `StartSpline`
  (params (SplineLocation :type "Vector Structure") (SplineRotation :type "Vector Structure") (`SplinePoint ` :type Integer))
  ;[0 0.09973 0.1094] Generate Spline
  ;;[1 1 1] Add New Spline Points At The Start
  (`/Engine/EditorBlueprintResources/StandardMacros.IncrementInt` `SplinePoint `
    (:`  `
      (`SplineComponent.AddSplinePoint` (`self.TerrainSpline`) (+ SplineLocation SplineRotation) "Local" true)
      (if (not (< `SplinePoint ` (+ (`self.StartInclineLenght`) 1)))
        (set `self.LevelStart` false)
        (set `self.SplineStart` true)))))

(event `DrawLine`
  (bind _returnvalue (- (`SplineComponent.GetNumberOfSplinePoints` (`self.TerrainSpline`)) 1))
  (bind _location (`SplineComponent.GetLocationAndTangentAtSplinePoint` (`self.TerrainSpline`) _returnvalue "Local"))
  ;[0 0.09973 0.1094] Generate Spline
  ;;[1 1 1] Loop for the first X spline points
  (for _ (range (+ (+ (`self.StartInclineLenght`) (`self.TotalSplineInOne`)) 1))
    (if (`self.LevelStart`)
      (`self.StartSpline` (`KismetMathLibrary.CreateVectorFromYawPitch` 90.0 (`KismetMathLibrary.RandomFloatInRange` -5.0 -20.0) 600.0) _location _returnvalue)
      (else
        (`self.NormalSpline` _location (`KismetMathLibrary.CreateVectorFromYawPitch` 90.0 (`KismetMathLibrary.RandomFloatInRange` -30.0 10.0) 800.0) _returnvalue))))
  (`self.Generate Mesh`)
  (`self.LastPos`))

(event `IsSplineGoingUp?`
  (bind _terrainspline (`self.TerrainSpline`))
  (bind _returnvalue (- (`SplineComponent.GetNumberOfSplinePoints` (`self.TerrainSpline`)) 1))
  (bind _z (.z (`SplineComponent.GetLocationAtSplinePoint` _terrainspline (- _returnvalue 1) "Local")))
  ;[0 0.09973 0.1094] Generate Spline
  ;;[1 1 1] Check if points in spline are going up
  (set `self.IsSplineGoingUp` (and (< (.z (`SplineComponent.GetLocationAtSplinePoint` _terrainspline _returnvalue "Local")) _z) (> _z (.z (`SplineComponent.GetLocationAtSplinePoint` _terrainspline (- _returnvalue 2) "Local"))))))

(fn `UserConstructionScript`)