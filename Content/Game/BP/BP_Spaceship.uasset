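; Player-controlled spaceship Blueprint that thrusts upward while the fly input is held, in a Flappy-style control scheme.
; BeginPlay registers the player Enhanced Input mapping context, and IA_Fly sets or clears the IsFlying flag.
; Each Tick, flying applies force along the collision's up vector and tilts the ship up; otherwise it tilts down.
; Each tilt direction stops once the ship's world roll passes its configured limit.
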(event `self.ReceiveBeginPlay`
  ;[1 1 1] Récupère IMC
  (bind _asplayer_controller (cast `PlayerController` (`self.GetController`)))
  (bind _returnvalue (pcsubsystem `EnhancedInputLocalPlayerSubsystem` _asplayer_controller))
  (`/Engine/EditorBlueprintResources/StandardMacros.IsValid` _returnvalue
    (:`Is Valid`
      (`EnhancedInputSubsystemInterface.AddMappingContext` _returnvalue "/Game/Game/PlayerInput/IMC_PlayerMouvement.IMC_PlayerMouvement" 1 (struct)))))

(event `self.ReceiveTick`
  (params (DeltaSeconds :type "Float (single-precision)"))
  ;[1 1 1] Tick
  (`self.Rotation Spaceship`))

(event `EnhancedInput|/Game/Game/PlayerInput/Input_Action/IA_Fly`
  (params (ActionValue :type Boolean) (ElapsedSeconds :type "Float (double-precision)") (TriggeredSeconds :type "Float (double-precision)") (InputAction :type "InputAction Object Reference" :default "/Game/Game/PlayerInput/Input_Action/IA_Fly.IA_Fly"))
  ;[1 1 1] Vérif si le joueur clique sur Fly
  (:`Started`
    (set `self.bIsFlying` true :!label _label))
  (:`Ongoing`
    (goto _label))
  (:`Canceled`
    (set `self.bIsFlying` false :!label _label_2)
    (set `self.bStopRotationUp` false)
    (set `self.bStopRotationDown` false))
  (:`Completed`
    (goto _label_2)))

(event `Rotation Up`
  (bind _spaceship (`self.Spaceship`))
  ;[1 1 1] Rotation Up
  (`SceneComponent.K2_AddLocalRotation` _spaceship (`self.RotationSpaceshipUp`) false false)
  (set `self.bStopRotationUp` (<= (.roll (`SceneComponent.K2_GetComponentRotation` _spaceship)) (`self.MaxRotationSpaceshipUp`))))

(event `Add Force Up`
  (bind _collision (`self.Collision`))
  ;[1 1 1] Force Up Spaceship
  (`PrimitiveComponent.AddForce` _collision (* (`SceneComponent.GetUpVector` _collision) (`self.fForce`)) "None" false))

(event `Rotation Down`
  (bind _spaceship (`self.Spaceship`))
  ;[1 1 1] Rotation Down
  (`SceneComponent.K2_AddLocalRotation` _spaceship (`self.RotationSpaceshipDown`) false false)
  (set `self.bStopRotationDown` (>= (.roll (`SceneComponent.K2_GetComponentRotation` _spaceship)) (`self.MaxRotationSpaceshipDown`))))

(event `Rotation Spaceship`
  ;[1 1 1] Rotation Spaceship
  (if (`self.bIsFlying`)
    (`self.Add Force Up`)
    (if (not (`self.bStopRotationUp`))
      (`self.Rotation Up`))
    (elif (not (`self.bStopRotationDown`))
      (`self.Rotation Down`))))

(fn `UserConstructionScript`)