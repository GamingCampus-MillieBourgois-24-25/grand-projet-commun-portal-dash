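; Portal actor in the snow level that moves the player to a randomly chosen Western or Space level.
; When the snow player overlaps its box, it destroys the snow level's obstacles, manager, killzones, terrain generation, colliders and power-ups.
; A one-time random pick then spawns that level's generators or managers and a wagon or spaceship pawn.
; It destroys the snow player, possesses the new pawn and gives itself a short lifespan.
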(event `ChangeLifeSpan`
  (`self.SetLifeSpan` 10.0))

(event `self.Box.OnComponentBeginOverlap`
  (params (OverlappedComponent :type "PrimitiveComponent Object Reference") (OtherActor :type "Actor Object Reference") (OtherComp :type "PrimitiveComponent Object Reference") (OtherBodyIndex :type Integer) (bFromSweep :type Boolean) (SweepResult :type "HitResult Structure (by ref)"))
  (bind _new_spawn (`self.New Spawn`))
  (bind _new_spawn_2 (`self.New Spawn`))
  (cast `/Game/Game/BP/BP_SnowPlayer` OtherActor)
  (`KismetSystemLibrary.PrintString` "portal")
  (`|ExecutionSequence`
    (:`then_0`
      (bind _outactors (`GameplayStatics.GetAllActorsOfClass` "/Game/Game/BP/Obstacles/BP_SnowObstacle.BP_SnowObstacle_C"))
      (`self.K2_DestroyActor` _outactors))
    (:`then_1`
      (bind _outactors_2 (`GameplayStatics.GetAllActorsOfClass` "/Game/Game/BP/BP_SnowGameManager.BP_SnowGameManager_C"))
      (`self.K2_DestroyActor` _outactors_2))
    (:`then_2`
      (bind _outactors_3 (`GameplayStatics.GetAllActorsOfClass` "/Game/Game/BP/BP_SnowKillzone.BP_SnowKillzone_C"))
      (`self.K2_DestroyActor` _outactors_3))
    (:`then_3`
      (bind _outactors_4 (`GameplayStatics.GetAllActorsOfClass` "/Game/Game/BP/BP_SnowTerrainGeneration.BP_SnowTerrainGeneration_C"))
      (`self.K2_DestroyActor` _outactors_4))
    (:`then_4`
      (bind _outactors_5 (`GameplayStatics.GetAllActorsOfClass` "/Game/Game/BP/BP_SnowGenerationCollider.BP_SnowGenerationCollider_C"))
      (`self.K2_DestroyActor` _outactors_5))
    (:`then_5`
      (bind _outactors_6 (`GameplayStatics.GetAllActorsOfClass` "/Game/Game/BP/PowerUps/BP_SnowPowerUps.BP_SnowPowerUps_C"))
      (`self.K2_DestroyActor` _outactors_6))
    (:`then_6`
      (`/Engine/EditorBlueprintResources/StandardMacros.DoOnce` false
        (:`Completed`
          (switch `int` (`KismetMathLibrary.RandomIntegerInRange` 0 1)
            (:`0`
              (`KismetSystemLibrary.PrintText` "Western")
              (bind _returnvalue (`|SpawnActorFromClass` "/Game/Game/BP/BP_Wagon.BP_Wagon_C" _new_spawn_2 "Undefined" "MultiplyWithRoot" null null))
              (set `self.NewPlayerPawn` _returnvalue)
              (`|SpawnActorFromClass` "/Game/Game/BP/BP_ObstableGeneratorWesternLevel.BP_ObstableGeneratorWesternLevel_C" _new_spawn_2 "Undefined" "MultiplyWithRoot" null null)
              (`|SpawnActorFromClass` "/Game/Game/BP/BP_CoinsManager.BP_CoinsManager_C" _new_spawn_2 "Undefined" "MultiplyWithRoot" null null)
              (`|SpawnActorFromClass` "/Game/Game/BP/BP_RailGeneratorLevelWestern.BP_RailGeneratorLevelWestern_C" _new_spawn_2 "Undefined" "MultiplyWithRoot" null null))
            (:`1`
              (`KismetSystemLibrary.PrintText` "Space")
              (`|SpawnActorFromClass` "/Game/Game/BP/Bp_ObstacleManager.Bp_ObstacleManager_C" _new_spawn "Undefined" "MultiplyWithRoot" null null)
              (`|SpawnActorFromClass` "/Game/Game/BP/BP_Slide_scrolling.BP_Slide_scrolling_C" _new_spawn "Undefined" "MultiplyWithRoot" null null)
              (bind _returnvalue_2 (`|SpawnActorFromClass` "/Game/Game/BP/BP_Spaceship.BP_Spaceship_C" _new_spawn "Undefined" "MultiplyWithRoot" null null))
              (set `self.NewPlayerPawn` _returnvalue_2)))
          (`self.PossesNewPawn`))))))

(event `PossesNewPawn`
  (bind _returnvalue (`GameplayStatics.GetActorOfClass` "/Game/Game/BP/BP_SnowPlayer.BP_SnowPlayer_C"))
  (`self.K2_DestroyActor` _returnvalue)
  (`Controller.Possess` (`GameplayStatics.GetPlayerController` 0) (`self.NewPlayerPawn`))
  (`self.ChangeLifeSpan`))

(fn `UserConstructionScript`)